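; UCenterCubeBP is an actor that casts a ring of line traces outward from its location when play begins.
; It rotates its forward vector around yaw in equal steps over a full circle, tracing on the Visibility channel out to Distance.
; The traces draw persistent debug lines, while an array write of each blocking-hit result is left unconnected and never runs.
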(event `Key|LeftShift`
  (params (Key :type "Key Structure")))

(event `self.ReceiveBeginPlay`
  (bind _returnvalue (`self.K2_GetActorLocation`))
  (bind _last_index (`self.Last Index`))
  (for _index (range (+ _last_index 1))
    (bind _outhit (`KismetSystemLibrary.LineTraceSingle` :`Start` _returnvalue :`End` (+ _returnvalue (* (`KismetMathLibrary.GreaterGreater_VectorRotator` (`self.GetActorForwardVector`) (`KismetMathLibrary.MakeRotator` 0.0 0.0 (* _index (/ 360.0 (`KismetMathLibrary.Conv_IntToDouble` (+ _last_index 1)))))) (`self.Distance`))) :`TraceChannel` "TraceTypeQuery1" :`DrawDebugType` "Persistent"))))

(fn `UserConstructionScript`)