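; DCenterCubeBP is a center cube that turns its surrounding pieces a quarter turn, like a Rubik's cube layer.
; Evenly spaced radial line traces find neighboring components and attach them to its static mesh, keeping world location and rotation.
; A timeline then lerps the mesh's relative yaw 90 degrees.
; DEvent or the D key turns it positive; RDEvent or the ReverseD action turns it negative.
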(event `DEvent`
  (bind _returnvalue (`self.K2_GetActorLocation`))
  (bind _last_index (`self.Last Index`))
  (bind _staticmeshcomponent (`self.StaticMeshComponent`))
  (for _index (range (+ _last_index 1)) :!label _label
    (bind _outhit (`KismetSystemLibrary.LineTraceSingle` _returnvalue (+ _returnvalue (* (`KismetMathLibrary.GreaterGreater_VectorRotator` (`self.GetActorForwardVector`) (`KismetMathLibrary.MakeRotator` 0.0 0.0 (* _index (/ 360.0 (`KismetMathLibrary.Conv_IntToDouble` (+ _last_index 1)))))) (`self.Distance`))) "TraceTypeQuery1"))
    (`SceneComponent.K2_AttachToComponent` (`.HitComponent` (`GameplayStatics.BreakHitResult` _outhit)) (`self.StaticMeshComponent`) "None" "KeepWorld" "KeepWorld" "KeepRelative" true))
  (bind _output_get (set `self.Relative Rotation` (`SceneComponent.RelativeRotation` _staticmeshcomponent)))
  (bind (_direction `_새_트랙_0`) (`Timeline|타임라인_0` :!via `PlayFromStart`)
    (:`Update`
      (`SceneComponent.K2_SetRelativeRotation` _staticmeshcomponent (`KismetMathLibrary.RLerp` _output_get (`KismetMathLibrary.MakeRotator` (.roll _output_get) (.pitch _output_get) (+ (.yaw _output_get) 90.0)) `_새_트랙_0` true) false false))))

(event `Key|D` :consume false
  (params (Key :type "Key Structure"))
  (:`Pressed`
    (goto _label)))

(event `RDEvent`
  (bind _returnvalue (`self.K2_GetActorLocation`))
  (bind _last_index (`self.Last Index`))
  (bind _staticmeshcomponent (`self.StaticMeshComponent`))
  (for _index (range (+ _last_index 1)) :!label _label_2
    (bind _outhit (`KismetSystemLibrary.LineTraceSingle` _returnvalue (+ _returnvalue (* (`KismetMathLibrary.GreaterGreater_VectorRotator` (`self.GetActorForwardVector`) (`KismetMathLibrary.MakeRotator` 0.0 0.0 (* _index (/ 360.0 (`KismetMathLibrary.Conv_IntToDouble` (+ _last_index 1)))))) (`self.Distance`))) "TraceTypeQuery1"))
    (`SceneComponent.K2_AttachToComponent` (`.HitComponent` (`GameplayStatics.BreakHitResult` _outhit)) (`self.StaticMeshComponent`) "None" "KeepWorld" "KeepWorld" "KeepRelative" true))
  (bind _output_get (set `self.Relative Rotation` (`SceneComponent.RelativeRotation` _staticmeshcomponent)))
  (bind (_direction `_새_트랙_0`) (`Timeline|타임라인_1` :!via `PlayFromStart`)
    (:`Update`
      (`SceneComponent.K2_SetRelativeRotation` _staticmeshcomponent (`KismetMathLibrary.RLerp` _output_get (`KismetMathLibrary.MakeRotator` (.roll _output_get) (.pitch _output_get) (+ (.yaw _output_get) -90.0)) `_새_트랙_0` true) false false))))

(event `InputAction|ReverseD` :consume false
  (params (Key :type "Key Structure"))
  (:`Pressed`
    (goto _label_2)))

(fn `UserConstructionScript`)